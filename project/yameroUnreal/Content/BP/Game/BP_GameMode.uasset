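; BP_GameMode is the game mode that drives the opening day-display and dialogue UI flow.
; On BeginPlay it shows the HUD_DisplayDay widget, then a ten-second timer calls GoToDayIDialogue by function name to remove it and create the HUD_Dialogue widget.
; It stores both widget references and exposes itself through the BPIGameModeRef function.
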(event `Create HUD Dialogue`
  (bind _returnvalue (`|CreateWidget` "/Game/BP/HUD/HUD_Dialogue.HUD_Dialogue_C"))
  (bind _output_get (set `self.HUD_dialogue Ref` _returnvalue))
  (`UserWidget.AddToViewport` _output_get 0))

(event `self.ReceiveBeginPlay`
  (bind _returnvalue (`|CreateWidget` "/Game/BP/HUD/HUD_DisplayDay.HUD_DisplayDay_C"))
  (bind _output_get (set `self.HUD_displayDay Ref` _returnvalue))
  (`UserWidget.AddToViewport` _output_get 0)
  (`KismetSystemLibrary.K2_SetTimer` null "GoToDayIDialogue" 10.0))

(event `GoToDayIDialogue`
  (`Widget.RemoveFromParent` (`self.HUD_displayDay Ref`))
  (`self.Create HUD Dialogue`))

(fn `BPI GameModeRef`
  (returns (`Game Mode Ref` :type "/Game/BP/Game/BP_GameMode Object Reference"))
  (return self))

(fn `UserConstructionScript`)